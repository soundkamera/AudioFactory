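; BP_Bullet is a bullet actor that damages what it touches and expires after five seconds if it hits nothing.
; Overlaps and hits both apply fixed damage, hide the mesh, spawn a stone impact particle and destroy the actor.
; Only the hit path adds a small force to its sphere and plays Wwise impact audio, setting a material switch from the surface type: concrete, metal, wood or human.
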(event `self.ReceiveBeginPlay`
  (`self.SetLifeSpan` 5.0))

(event `self.ReceiveActorBeginOverlap`
  (params (OtherActor :type "Actor Object Reference"))
  (`GameplayStatics.ApplyDamage` OtherActor 20.0)
  (`SceneComponent.SetVisibility` (`self.Bullet`) false false)
  (`GameplayStatics.SpawnEmitterAtLocation` "/Game/AudioRG/AudioFactoryAssets/Shooting/Weapons/Bullet/P_Impact_Stone_Small_01.P_Impact_Stone_Small_01" (`self.K2_GetActorLocation`))
  (`self.K2_DestroyActor`))

(event `self.ReceiveHit`
  (params (MyComp :type "PrimitiveComponent Object Reference") (Other :type "Actor Object Reference") (OtherComp :type "PrimitiveComponent Object Reference") (bSelfMoved :type Boolean) (HitLocation :type "Vector Structure") (HitNormal :type "Vector Structure") (NormalImpulse :type "Vector Structure") (Hit :type "HitResult Structure (by ref)"))
  (`|ExecutionSequence`
    (:`then_0`
      (`GameplayStatics.ApplyDamage` Other 20.0)
      (`PrimitiveComponent.AddForceAtLocation` (`self.Sphere`) (1.0 1.0 1.0) HitLocation "None")
      (`SceneComponent.SetVisibility` (`self.Bullet`) false false)
      (`GameplayStatics.SpawnEmitterAtLocation` "/Game/AudioRG/AudioFactoryAssets/Shooting/Weapons/Bullet/P_Impact_Stone_Small_01.P_Impact_Stone_Small_01" (`self.K2_GetActorLocation`)))
    (:`then_1`
      (switch `EPhysicalSurface` (`GameplayStatics.GetSurfaceType` Hit)
        (:`SurfaceType1`
          (`AkGameplayStatics.SetSwitch` "/Game/WwiseAudio/Switches/Default_Work_Unit/BULLET_IMPACTS_Materials/BULLET_IMPACTS_Materials-CONCRETE.BULLET_IMPACTS_Materials-CONCRETE" self))
        (:`SurfaceType2`
          (`AkGameplayStatics.SetSwitch` "/Game/WwiseAudio/Switches/Default_Work_Unit/BULLET_IMPACTS_Materials/BULLET_IMPACTS_Materials-METAL.BULLET_IMPACTS_Materials-METAL" self))
        (:`SurfaceType3`
          (`AkGameplayStatics.SetSwitch` "/Game/WwiseAudio/Switches/Default_Work_Unit/BULLET_IMPACTS_Materials/BULLET_IMPACTS_Materials-WOOD.BULLET_IMPACTS_Materials-WOOD" self))
        (:`SurfaceType4`
          (`AkGameplayStatics.SetSwitch` "/Game/WwiseAudio/Switches/Default_Work_Unit/BULLET_IMPACTS_Materials/BULLET_IMPACTS_Materials-HUMAN.BULLET_IMPACTS_Materials-HUMAN" self)))
      (`AkGameplayStatics.PostEvent` "/Game/WwiseAudio/Events/SFX_Events/Play_Bullet_Impact.Play_Bullet_Impact" self))
    (:`then_2`
      (`self.K2_DestroyActor`))))

(fn `UserConstructionScript`)