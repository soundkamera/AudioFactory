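; Physical prop actor that plays a Wwise impact sound when its static mesh hits something.
; On hit, the hit component's speed, if above a minimum, is remapped into the Collision_Velocity RTPC before Play_Impact posts on the actor.
; A DoOnce reset after a short delay throttles repeated impacts, and the mapped value is printed on screen for debugging.
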(event `self.StaticMeshComponent.OnComponentHit`
  (params (HitComponent :type "PrimitiveComponent Object Reference") (OtherActor :type "Actor Object Reference") (OtherComp :type "PrimitiveComponent Object Reference") (NormalImpulse :type "Vector Structure") (Hit :type "HitResult Structure (by ref)"))
  (bind _returnvalue (`KismetMathLibrary.VSize` (`SceneComponent.GetComponentVelocity` HitComponent)))
  (bind _returnvalue_2 (`KismetMathLibrary.MapRangeClamped` _returnvalue 0.0 400.0 0.0 100.0))
  (`|ExecutionSequence`
    (:`then_0`
      (`/Engine/EditorBlueprintResources/StandardMacros.DoOnce` false :!label _label
        (:`Completed`
          (`KismetSystemLibrary.PrintString` (`KismetStringLibrary.Conv_DoubleToString` _returnvalue_2) true true (struct :`G` 0.66 :`B` 1.0 :`A` 1.0) 20.0)
          (if (>= _returnvalue 40.0)
            (`AkGameplayStatics.SetRTPCValue` "/Game/WwiseAudio/Game_Parameters/Default_Work_Unit/Collision_Velocity.Collision_Velocity" _returnvalue_2)
            (`AkGameplayStatics.PostEvent` "/Game/WwiseAudio/Events/SFX_Events/Play_Impact.Play_Impact" self)))))
    (:`then_1`
      (`KismetSystemLibrary.Delay` 0.2)
      (goto _label :!via `Reset`))))

(fn `UserConstructionScript`)