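; Anim notify that plays Wwise footstep audio matched to the surface beneath the animated mesh's owner.
; It line-traces downward from the owner on the Visibility channel and maps concrete or metal plate physical surfaces to a Wwise switch.
; The switch and the single Play_Footstep_L event target player character 0 rather than the notifying actor.
; Other surfaces have no handling.
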(fn `Received_Notify`
  (params (MeshComp :type "SkeletalMeshComponent Object Reference") (Animation :type "AnimSequenceBase Object Reference") (EventReference :type "AnimNotifyEventReference Structure (by ref)"))
  (returns (ReturnValue :type Boolean))
  (bind _returnvalue (`ActorComponent.GetOwner` MeshComp))
  (bind _returnvalue_2 (`GameplayStatics.GetPlayerCharacter` 0))
  (bind _returnvalue_3 (`Actor.K2_GetActorLocation` _returnvalue))
  (bind (_outhit _returnvalue_4) (`KismetSystemLibrary.LineTraceSingle` _returnvalue_3 (+ _returnvalue_3 (* (`Actor.GetActorUpVector` _returnvalue) (0.0 0.0 -200.0))) "TraceTypeQuery1"))
  (if _returnvalue_4
    (switch `EPhysicalSurface` (`GameplayStatics.GetSurfaceType` _outhit)
      (:`SurfaceType1`
        (`AkGameplayStatics.SetSwitch` "/Game/WwiseAudio/Switches/Default_Work_Unit/SURFACES/SURFACES-CONCRETE.SURFACES-CONCRETE" _returnvalue_2))
      (:`SurfaceType2`
        (`AkGameplayStatics.SetSwitch` "/Game/WwiseAudio/Switches/Default_Work_Unit/SURFACES/SURFACES-METAL_PLATE.SURFACES-METAL_PLATE" _returnvalue_2)))
    (`AkGameplayStatics.PostEvent` "/Game/WwiseAudio/Events/FOL_Events/Play_Footstep_L.Play_Footstep_L" _returnvalue_2)
    (return false)))